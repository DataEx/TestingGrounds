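; AI controller for guard NPCs that sets up the PatrolData blackboard and runs the GuardBehavior tree.
; AI perception stores sensed actors lacking an AI controller as the Enemy key and clears it when sensing fails, printing their names.
; Each tick, it sets the pawn's TP_Character Aiming and Shooting flags according to whether the controller has a valid focus actor.
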(event OnTargetPerceptionUpdated(AIPerception)
  (params (Actor :type Actor%20Object%20Reference) (Stimulus :type AI%20Stimulus%20Structure))
  (bind _returnvalue (Utilities|Name|MakeLiteralName "Enemy"))
  (bind _blackboardcomp (Variables|Default|GetBlackboardComp))
  (Utilities|IsValid (AI|GetAIController Actor)
    (:Is%20Not%20Valid
      (Development|PrintString (Utilities|GetDisplayName Actor))
      (if (.bSuccessfullySensed (Utilities|Struct|BreakAIStimulus Stimulus))
        (AI|Components|Blackboard|SetValueasObject _blackboardcomp _returnvalue Actor)
        (else
          (AI|Components|Blackboard|ClearValue _blackboardcomp _returnvalue))))))

(event EventBeginPlay
  ;[1 1 1] Initialize blackboard
  (bind _blackboardcomponent (Class|AIController|UseBlackboard "/Game/NPC/AI/PatrolData.PatrolData"))
  (Variables|Default|SetBlackboardComp _blackboardcomponent)
  (AI|RunBehaviorTree "/Game/NPC/AI/GuardBehavior.GuardBehavior"))

(event EventTick
  (params (DeltaSeconds :type Float%20%28single-precision%29))
  (bind _returnvalue (Class|AIController|GetFocusActor))
  (bind _returnvalue_2 (Utilities|IsValid _returnvalue))
  (bind _astp_character (Utilities|Casting|CastToTP_Character (Pawn|GetControlledPawn)))
  (Variables|/Game/NPC/Behavior/TP_Character.TP_Character_C|SetAiming _astp_character _returnvalue_2)
  (Variables|/Game/NPC/Behavior/TP_Character.TP_Character_C|SetShooting _astp_character _returnvalue_2))

(fn ConstructionScript)