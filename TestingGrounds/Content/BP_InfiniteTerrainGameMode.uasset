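; Game mode for an infinite terrain game that chains tiles end to end and keeps score.
; On BeginPlay it populates a nav mesh bounds volume pool, then spawns an initial run of tiles.
; SpawnNextTile passes that pool to each new BP_Tile and stores its attach location as the next spawn transform.
; NewTileConquered increments the score, which GetScore returns.
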(event EventBeginPlay
  (Class|InfiniteTerrainGameMode|PopulateBoundsVolumePool)
  (for _index (range 0 3)
    (CallFunction|SpawnNextTile)))

(fn ConstructionScript)

(fn SpawnNextTile
  (bind _returnvalue (Game|SpawnActorfromClass "/Game/Levels/Terrain/BP_Tile.BP_Tile_C" (Variables|Default|GetPreviousTileTransform) "Undefined" 0 0))
  (Class|Tile|SetPool _returnvalue (Variables|Default|GetNavMeshBoundsVolumePool))
  (bind _attachtransform (Default|GetAttachLocation _returnvalue))
  (Variables|Default|SetPreviousTileTransform _attachtransform))

(fn NewTileConquered
  (Math|Integer|IncrementInt (Variables|Default|GetScore)))

(fn GetScore
  (return (Variables|Default|GetScore)))